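; BP_IndraArrow is an arrow projectile, named for Indra, that is launched on demand and damages what it overlaps.
; Fire adds a projectile movement component at runtime, interpolating speed and gravity scale from shot strength, and attaches an ultimate arrow particle effect.
; Arrow overlap sends a fixed-damage TakeDamage message to the other actor without filtering or destroying itself; the Box overlap and hit events are empty.
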(event OnComponentBeginOverlap(arrow)
  (params (OverlappedComponent :type Primitive%20Component%20Object%20Reference) (OtherActor :type Actor%20Object%20Reference) (OtherComp :type Primitive%20Component%20Object%20Reference) (OtherBodyIndex :type Integer) (bFromSweep :type Boolean) (SweepResult :type Hit%20Result%20Structure%20%28by%20ref%29))
  (Class|BPDamagable|TakeDamage(Message) OtherActor (Utilities|Struct|MakeS_Damage_Info 2e+01 "NewEnumerator1" "NewEnumerator4" false false false false)))

(event OnComponentBeginOverlap(Box)
  (params (OverlappedComponent :type Primitive%20Component%20Object%20Reference) (OtherActor :type Actor%20Object%20Reference) (OtherComp :type Primitive%20Component%20Object%20Reference) (OtherBodyIndex :type Integer) (bFromSweep :type Boolean) (SweepResult :type Hit%20Result%20Structure%20%28by%20ref%29)))

(event OnComponentHit(Box)
  (params (HitComponent :type Primitive%20Component%20Object%20Reference) (OtherActor :type Actor%20Object%20Reference) (OtherComp :type Primitive%20Component%20Object%20Reference) (NormalImpulse :type Vector :default "0, 0, 0") (Hit :type Hit%20Result%20Structure%20%28by%20ref%29)))

(event Custom|Fire
  (params (Direction :type Vector) (Strength :type Float%20%28double-precision%29))
  (bind _returnvalue (AddComponent|AddProjectileMovementComponent))
  (Variables|/Script/Engine.MovementComponent|SetVelocity _returnvalue (* Direction (Math|Float|Lerp (Variables|Default|GetMinSpeed) (Variables|Default|GetMaxSpeed) Strength)))
  (Variables|/Script/Engine.ProjectileMovementComponent|SetProjectileGravityScale _returnvalue (Math|Float|Lerp (Variables|Default|GetMaxGravity) (Variables|Default|GetMinGravity) Strength))
  (Effects|SpawnEmitterAttached "/Game/assets/P_Arrow_Ultimate.P_Arrow_Ultimate" (Variables|Default|GetScene) "None" "0, 0, 0" "0, 0, 0" "0.500000,0.500000,0.500000"))

(event EventBeginPlay)

(event Collision|EventActorBeginOverlap
  (params (OtherActor :type Actor%20Object%20Reference)))

(event EventTick
  (params (DeltaSeconds :type Float%20%28single-precision%29)))

(fn ConstructionScript)