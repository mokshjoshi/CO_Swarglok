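; Base enemy character that exposes health, damage, patrol route, movement speed and combat range functions for AI and combat.
; Health, healing and damage are delegated to the BPCDamage component, and a health bar widget is bound to the actor.
; On hit, it stops, freezes its AI controller's state and plays a react montage before resuming attack on the last known target.
; Death enables mesh ragdoll physics and stops the AI logic.
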(event OnComponentBeginOverlap(Mesh)
  (params (OverlappedComponent :type Primitive%20Component%20Object%20Reference) (OtherActor :type Actor%20Object%20Reference) (OtherComp :type Primitive%20Component%20Object%20Reference) (OtherBodyIndex :type Integer) (bFromSweep :type Boolean) (SweepResult :type Hit%20Result%20Structure%20%28by%20ref%29)))

(event Custom|OnDeath_Event
  (bind _mesh (Variables|Character|GetMesh))
  (bind _as_aic_enemy_base (Variables|Default|GetAs%20AIC%20Enemy%20Base))
  (Physics|SetSimulatePhysics _mesh true)
  (Collision|SetCollisionEnabled _mesh "QueryAndPhysics")
  (AI|Logic|StopLogic (Variables|/Script/AIModule.AIController|GetBrainComponent _as_aic_enemy_base) "")
  (Default|SetStateasDead _as_aic_enemy_base))

(event Custom|HitResponseEvent
  (params (DamageResponse :type EN_Damage_Response%20Enum :default "NewEnumerator0"))
  (Components|Movement|StopMovementImmediately (Variables|Character|GetCharacterMovement))
  (Default|SetStateasFrozen (Variables|Default|GetAs%20AIC%20Enemy%20Base))
  (Animation|Montage|PlayMontage (Variables|Character|GetMesh) (Variables|Default|GetHitReact)
    (:OnCompleted
      _)
    (:OnInterrupted
      _))
  (Default|SetStateasAttacking (Variables|Default|GetAs%20AIC%20Enemy%20Base) 0 true))

(event EventBeginPlay
  (bind _bpc_damage (Variables|Default|GetBPC_Damage))
  (bind _asaic_enemy_base (Utilities|Casting|CastToAIC_EnemyBase (AI|GetAIController self)))
  (Variables|Default|SetAs%20AIC%20Enemy%20Base _asaic_enemy_base)
  (bind _returnvalue (UserInterface|CreateWidget "/Game/DamageSystem/WB_HealthBar111.WB_HealthBar111_C" 0 self))
  (UserInterface|SetWidget (Variables|Default|GetHealthBar) _returnvalue)
  (EventDispatchers|AssignOnDeath _bpc_damage (delegate Custom|OnDeath_Event))
  (EventDispatchers|AssignOnDamageResonse _bpc_damage (EventDispatchers|CreateEvent :!event Custom|HitResponseEvent)))

(event Game|Damage|EventAnyDamage
  (params (Damage :type Float%20%28single-precision%29) (DamageType :type Damage%20Type%20Object%20Reference) (InstigatedBy :type Controller%20Object%20Reference) (DamageCauser :type Actor%20Object%20Reference)))

(fn ConstructionScript
  (bind _bpc_damage (Variables|Default|GetBPC_Damage))
  (Variables|/Game/DamageSystem/BPC_Damage.BPC_Damage_C|SetMaxHealth _bpc_damage 1e+02)
  (Variables|/Game/DamageSystem/BPC_Damage.BPC_Damage_C|SetHealth _bpc_damage 1e+02))

(fn GetCurrentHealth
  (return (Variables|/Game/DamageSystem/BPC_Damage.BPC_Damage_C|GetHealth (Variables|Default|GetBPC_Damage))))

(fn GetIdealRamge
  (return 1.5e+02 3e+02))

(fn GetMaxHealth
  (return (Variables|/Game/DamageSystem/BPC_Damage.BPC_Damage_C|GetMaxHealth (Variables|Default|GetBPC_Damage))))

(fn GetPatrolRoute
  (return (Variables|AI|GetPatrolRoute)))

(fn Heal
  (params (Amount :type Float%20%28double-precision%29))
  (bind _newhealth (Default|Heal (Variables|Default|GetBPC_Damage) Amount))
  (return _newhealth))

(fn IsDead
  (return (Variables|/Game/DamageSystem/BPC_Damage.BPC_Damage_C|GetIs%20Dead? (Variables|Default|GetBPC_Damage))))

(fn SetMovementSpeed
  (params (Speed :type E_MovementSpeed%20Enum :default "NewEnumerator0"))
  (Variables|/Script/Engine.CharacterMovementComponent|SetMaxWalkSpeed (Variables|Character|GetCharacterMovement) (Utilities|Select :Index Speed :NewEnumerator0 0.0 :NewEnumerator1 1e+02 :NewEnumerator2 3e+02 :NewEnumerator3 5e+02))
  (return 0.0))

(fn TakeDamage
  (params (DamageInfo :type S%20Damage%20Info%20Structure))
  (bind _wasdamaged_ (Default|TakeDamage (Variables|Default|GetBPC_Damage) DamageInfo))
  (return _wasdamaged_))