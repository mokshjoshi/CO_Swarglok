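; BP_Indra is a ranged, teleporting enemy character driven by an AI controller.
; Attack plays a fireball montage whose notify line-traces to the controller's AttackTarget and applies instant damage, with no projectile.
; Teleport is really a very fast flying AIMoveTo with hidden mesh, pawn collision ignored and attached particle trails, all reverted on arrival or failure.
; It signals attack and teleport completion, and supplies movement speeds and ideal combat ranges.
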(event Custom|Teleport
  (params (Location :type Vector))
  (bind _charactermovement (Variables|Character|GetCharacterMovement))
  (if (not (Variables|Default|GetISTeleporting))
    (Variables|Default|SetISTeleporting true)
    (Pawn|Components|CharacterMovement|SetMovementMode _charactermovement "MOVE_Flying" 0)
    (Variables|/Script/Engine.CharacterMovementComponent|SetMaxFlySpeed _charactermovement 8e+03)
    (Variables|/Script/Engine.CharacterMovementComponent|SetMaxAcceleration _charactermovement 99999.0)
    (Rendering|SetVisibility (Variables|Character|GetMesh) false true)
    (Collision|SetCollisionResponsetoChannel (Variables|Default|GetCapsuleComponent) "ECC_Pawn" "ECR_Ignore")
    (bind _returnvalue (Effects|SpawnEmitterAttached "/Game/3d/Swarglok/burrrrr.burrrrr" (Variables|Character|GetMesh) "Spine1" "0, 0, 0" "0, 0, 0" "0.800000,0.800000,0.800000"))
    (Variables|Default|SetTeleportBodyEffect _returnvalue)
    (bind _returnvalue_2 (Effects|SpawnEmitterAttached "/Game/3d/Swarglok/meteorrrrrrrr.meteorrrrrrrr" (Variables|Character|GetMesh) "Spine1"))
    (Variables|Default|SetTeleport%20Trail _returnvalue_2)
    (Animation|StopAnimMontage 0)
    (AI|AIMoveTo self Location 0 15.0 false
      (:OnSuccess
        _)
      (:OnFail
        _))
    (CallFunction|TeleportEnd)
    (else
      (Utilities|FlowControl|DelayUntilNextTick)
      (Default|CallOnTeleportEnd))))

(event Custom|Teleport%20End
  (bind _charactermovement (Variables|Character|GetCharacterMovement))
  (Components|Movement|StopMovementImmediately (Variables|Character|GetCharacterMovement))
  (Pawn|Components|CharacterMovement|SetMovementMode _charactermovement "MOVE_Walking" 0)
  (Variables|/Script/Engine.CharacterMovementComponent|SetMaxAcceleration _charactermovement 1.5e+03)
  (Rendering|SetVisibility (Variables|Character|GetMesh) true true)
  (Collision|SetCollisionResponsetoChannel (Variables|Default|GetCapsuleComponent) "ECC_Pawn" "ECR_Block")
  (Default|CallOnTeleportEnd)
  (Utilities|FlowControl|Delay 0.5)
  (Variables|Default|SetISTeleporting false)
  (Utilities|FlowControl|Sequence
    (:then_0
      (bind _teleportbodyeffect (Variables|Default|GetTeleportBodyEffect)
        (:then
          (Components|DestroyComponent _teleportbodyeffect))
        (:else)))
    (:then_1
      (bind _teleport_trail (Variables|Default|GetTeleport%20Trail)
        (:then
          (Components|DestroyComponent _teleport_trail))
        (:else)))))

(event EventBeginPlay
  (|CallParentFunction) ; This node is disabled and will not be called.\nDrag off pins to build functionality.
)

(event Collision|EventActorBeginOverlap
  (params (OtherActor :type Actor%20Object%20Reference)))

(event EventTick
  (params (DeltaSeconds :type Float%20%28single-precision%29)))

(event EventAttack
  (bind _notifyname (Animation|Montage|PlayMontage (Variables|Character|GetMesh) "/Game/3d/Swarglok/Animations/Fireball_Montage.Fireball_Montage")
    (:OnCompleted
      (Default|CallOnAttackEnd :!label _label))
    (:OnInterrupted
      (goto _label))
    (:OnNotifyBegin
      (switch name _notifyname
        (:Fire
          (bind _asaic_enemy_base (Utilities|Casting|CastToAIC_EnemyBase (AI|GetAIController self)))
          (bind _attacktarget (Variables|/Game/Enemies/AI/AIC_EnemyBase.AIC_EnemyBase_C|GetAttackTarget _asaic_enemy_base)
            (:then
              (bind (_outhit _returnvalue) (Collision|LineTraceForObjects (Transformation|GetActorLocation) (Transformation|GetActorLocation _attacktarget) (Utilities|Array|MakeArray "ObjectTypeQuery3") false 0 "None"))
              (if _returnvalue
                (Game|Damage|ApplyDamage (.HitActor (Collision|BreakHitResult _outhit)) 2e+01 0 0)))
            (:else)))))))

(fn ConstructionScript
  (|CallParentFunction))

(fn SetMovementSpeed
  (params (Speed :type E_MovementSpeed%20Enum :default "NewEnumerator0"))
  (return (Utilities|Select :Index Speed :NewEnumerator0 0.0 :NewEnumerator1 1.5e+02 :NewEnumerator2 2.5e+02 :NewEnumerator3 4e+02)))

(fn GetIdealRamge
  (return 5e+02 7e+02))