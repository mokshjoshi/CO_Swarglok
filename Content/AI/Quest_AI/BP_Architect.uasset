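; BP_Architect is a quest-giver NPC character that shows an interact prompt while the player is inside its sphere.
; InteractFn toggles a WB_QuestGiver widget, filling it from the Quest array, passing itself as the giver and switching mouse cursor and input mode.
; Clap and sad montage events play right or wrong answer animations, each with a matching feedback widget shown for 1.5 seconds.
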(event OnComponentBeginOverlap(Sphere)
  (params (OverlappedComponent :type Primitive%20Component%20Object%20Reference) (OtherActor :type Actor%20Object%20Reference) (OtherComp :type Primitive%20Component%20Object%20Reference) (OtherBodyIndex :type Integer) (bFromSweep :type Boolean) (SweepResult :type Hit%20Result%20Structure%20%28by%20ref%29))
  ;[0.002081 0.07315 0.15 0.5] Press e on overrlap
  (Utilities|Casting|CastToBP_ThirdPersonCharacter OtherActor)
  (UserInterface|Viewport|AddtoViewport (Variables|Default|GetNewVar) 0))

(event OnComponentEndOverlap(Sphere)
  (params (OverlappedComponent :type Primitive%20Component%20Object%20Reference) (OtherActor :type Actor%20Object%20Reference) (OtherComp :type Primitive%20Component%20Object%20Reference) (OtherBodyIndex :type Integer))
  ;[0.002081 0.07315 0.15 0.5] Press e on overrlap
  (Utilities|Casting|CastToBP_ThirdPersonCharacter OtherActor)
  (Widget|RemovefromParent (Variables|Default|GetNewVar)))

(event Custom|Close%20widget
  (bind _returnvalue (Game|GetPlayerController 0))
  ;[0.01717 0 0.15 0.5] Quest widget logic
  (Widget|RemovefromParent (Variables|Default|GetQuests%20Widget))
  (Variables|Default|SetQuests%20Widget 0)
  (Variables|Default|SetWidget%20active false)
  (Variables|/Script/Engine.PlayerController|SetbShowMouseCursor _returnvalue false)
  (Input|SetInputModeGameOnly _returnvalue false))

(event Custom|PLAY%20Clap%20Montage
  (Animation|PlayAnimMontage "/Game/Assets/RTG_/RTG_Clapping_Montage.RTG_Clapping_Montage" 1.0 "None")
  (bind _returnvalue (UserInterface|CreateWidget "/Game/AI/Quest_AI/WB_RightAnswer.WB_RightAnswer_C"))
  (UserInterface|Viewport|AddtoViewport _returnvalue 0)
  (Utilities|FlowControl|Delay 1.5)
  (Widget|RemovefromParent _returnvalue))

(event Custom|Play%20sad%20Montage
  (Animation|PlayAnimMontage "/Game/Assets/RTG_/RTG_Annoyed_Head_Shake_Montage.RTG_Annoyed_Head_Shake_Montage" 1.0 "None")
  (bind _returnvalue (UserInterface|CreateWidget "/Game/AI/Quest_AI/WB_WrongAnswer.WB_WrongAnswer_C"))
  (UserInterface|Viewport|AddtoViewport _returnvalue 0)
  (Utilities|FlowControl|Delay 1.5)
  (Widget|RemovefromParent _returnvalue))

(event EventBeginPlay
  (bind _returnvalue (UserInterface|CreateWidget "/Game/AI/Quest_AI/Interact.Interact_C"))
  (Variables|Default|SetNewVar _returnvalue)
  (bind _returnvalue_2 (UserInterface|CreateWidget "/Game/AI/Quest_AI/WBP_QuestObjectiveSlot.WBP_QuestObjectiveSlot_C"))
  (Variables|Default|Setoptions _returnvalue_2)
  (bind _asbp_third_person_character (Utilities|Casting|CastToBP_ThirdPersonCharacter (Game|GetPlayerCharacter 0)))
  (Variables|Default|SetAs%20BP%20Third%20Person%20Character _asbp_third_person_character))

(event Collision|EventActorBeginOverlap
  (params (OtherActor :type Actor%20Object%20Reference)))

(event EventTick
  (params (DeltaSeconds :type Float%20%28single-precision%29)))

(event EventInteractFn
  (bind _returnvalue (Game|GetPlayerController 0))
  (bind _returnvalue_2 (Game|GetPlayerController 0))
  ;[0.01717 0 0.15 0.5] Quest widget logic
  (Widget|RemovefromParent (Variables|Default|GetNewVar))
  (if (not (Variables|Default|GetWidget%20active))
    (bind _returnvalue_3 (UserInterface|CreateWidget "/Game/AI/Quest_AI/WB_QuestGiver.WB_QuestGiver_C"))
    (bind _output_get (Variables|Default|SetQuests%20Widget _returnvalue_3))
    (UserInterface|Viewport|AddtoViewport _output_get 0)
    (Variables|Default|SetWidget%20active true)
    (Variables|/Script/Engine.PlayerController|SetbShowMouseCursor _returnvalue true)
    (Input|SetInputModeGameandUI _returnvalue (Variables|Default|GetQuests%20Widget) "DoNotLock" true false)
    (Variables|/Game/AI/Quest_AI/WB_QuestGiver.WB_QuestGiver_C|SetQuest%20giver%20bp (Variables|Default|GetQuests%20Widget) self)
    (for _array_element (Variables|Default|GetQuest)
      (Default|AddQuest (Variables|Default|GetQuests%20Widget) _array_element))
    (else
      (UserInterface|Viewport|AddtoViewport (Variables|Default|GetNewVar) 0)
      (Widget|RemovefromParent (Variables|Default|GetQuests%20Widget))
      (Variables|Default|SetQuests%20Widget 0)
      (Variables|Default|SetWidget%20active false)
      (Variables|/Script/Engine.PlayerController|SetbShowMouseCursor _returnvalue_2 false)
      (Input|SetInputModeGameOnly _returnvalue_2 false))))

(fn ConstructionScript)