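; Civilian NPC that wanders random reachable points, offers random dialogue to the player and can be killed.
; A box overlap with the player shows an interact prompt, and the interact event flip-flops between a dialogue widget and resumed roaming.
; Zero health from AnyDamage or any of three arrow types triggers ragdoll, with arrow kills destroyed after a delay.
; Damage interface functions partly forward to BPCDamage, while IsDead and Heal are stubs.
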(event OnComponentBeginOverlap(col)
  (params (OverlappedComponent :type Primitive%20Component%20Object%20Reference) (OtherActor :type Actor%20Object%20Reference) (OtherComp :type Primitive%20Component%20Object%20Reference) (OtherBodyIndex :type Integer) (bFromSweep :type Boolean) (SweepResult :type Hit%20Result%20Structure%20%28by%20ref%29))
  (Utilities|FlowControl|Sequence
    (:then_0
      (Utilities|Casting|CastToBP_Arrow OtherActor)
      (CallFunction|Die)
      (AI|AIMoveTo self "0, 0, 0" 0 5.0 false
        (:then
          (Utilities|FlowControl|Delay 1e+01)
          (Actor|DestroyActor))))
    (:then_1
      (Utilities|Casting|CastToBP_IndraArrow OtherActor)
      (CallFunction|Die)
      (AI|AIMoveTo self "0, 0, 0" 0 5.0 false
        (:then
          (Utilities|FlowControl|Delay 1e+01)
          (Actor|DestroyActor))))
    (:then_2
      (Utilities|Casting|CastToBP_VarunArrow OtherActor)
      (CallFunction|Die)
      (AI|AIMoveTo self "0, 0, 0" 0 5.0 false
        (:then
          (Utilities|FlowControl|Delay 1e+01)
          (Actor|DestroyActor))))))

(event OnComponentBeginOverlap(Box)
  (params (OverlappedComponent :type Primitive%20Component%20Object%20Reference) (OtherActor :type Actor%20Object%20Reference) (OtherComp :type Primitive%20Component%20Object%20Reference) (OtherBodyIndex :type Integer) (bFromSweep :type Boolean) (SweepResult :type Hit%20Result%20Structure%20%28by%20ref%29))
  ;[0 0.008249 0.15 0.5] On Overlap
  (Utilities|Casting|CastToBP_ThirdPersonCharacter OtherActor)
  (Variables|Default|Setis%20overlapped%20with%20box? true)
  (UserInterface|Viewport|AddtoViewport (Variables|Default|GetWB_Interact) 0))

(event OnComponentEndOverlap(Box)
  (params (OverlappedComponent :type Primitive%20Component%20Object%20Reference) (OtherActor :type Actor%20Object%20Reference) (OtherComp :type Primitive%20Component%20Object%20Reference) (OtherBodyIndex :type Integer))
  ;[0 0.008249 0.15 0.5] On Overlap
  (Utilities|Casting|CastToBP_ThirdPersonCharacter OtherActor)
  (Variables|Default|Setis%20overlapped%20with%20box? false)
  (Variables|Default|SetDailogue%20shown false)
  (Widget|RemovefromParent (Variables|Default|GetWB_Interact))
  (CallFunction|RandomRoam)
  (Widget|RemovefromParent (Variables|Default|GetWB_Dailogue)))

(event Custom|HitResponseEvent
  (params (DamageResponse :type EN_Damage_Response%20Enum :default "NewEnumerator0"))
  (Components|Movement|StopMovementImmediately (Variables|Character|GetCharacterMovement))
  (Animation|Montage|PlayMontage (Variables|Character|GetMesh) (Variables|Default|GetHitReact)))

(event Custom|Die
  (bind _mesh (Variables|Character|GetMesh))
  (Physics|SetSimulatePhysics _mesh true)
  (Collision|SetCollisionEnabled _mesh "QueryAndPhysics"))

(event Custom|RandomRoam
  ;[0 0.01831 0.15 0.5] Begin Play
  (if (not (Variables|Default|GethasInteracted>))
    (AI|AIMoveTo self (.RandomLocation (AI|Navigation|GetRandomReachablePointinRadius (Transformation|GetActorLocation) (Variables|Default|Getroaming%20Radius) 0 0)) 0 5.0 false
      (:OnSuccess
        (Utilities|FlowControl|Delay 0.2)
        (CallFunction|RandomRoam)))))

(event EventInteractwithCivilillian
  ;[0 0.007824 0.15 0.5] Interaction logic
  (Utilities|FlowControl|FlipFlop
    (:A
      (if (and (Variables|Default|Getis%20overlapped%20with%20box?) (not (Variables|Default|GetDailogue%20shown)))
        _
        (else
          _))
      (Variables|/Script/UMG.TextBlock|SetText (Variables|/Game/AI/Civilian/Dailogue.Dailogue_C|GetDailoguetext (Variables|Default|GetWB_Dailogue)) (Utilities|Text|ToText(String) (Utilities|Array|Get(acopy) (Variables|Default|GetDailogue) (Math|Random|RandomIntegerinRange 0 (Variables|Default|Getdailogue%20index)))))
      (UserInterface|Viewport|AddtoViewport (Variables|Default|GetWB_Dailogue) 0)
      (Variables|Default|SetDailogue%20shown true)
      (Widget|RemovefromParent (Variables|Default|GetWB_Interact))
      (AI|AIMoveTo self "0, 0, 0" 0 5.0 false))
    (:B
      (CallFunction|RandomRoam)
      (UserInterface|Viewport|AddtoViewport (Variables|Default|GetWB_Interact) 0)
      (Widget|RemovefromParent (Variables|Default|GetWB_Dailogue)))))

(event EventBeginPlay
  (CallFunction|RandomRoam)
  (bind _returnvalue (UserInterface|CreateWidget "/Game/AI/Civilian/Dailogue.Dailogue_C"))
  (Variables|Default|SetWB_Dailogue _returnvalue)
  (bind _returnvalue_2 (UserInterface|CreateWidget "/Game/AI/Quest_AI/Interact.Interact_C"))
  (Variables|Default|SetWB_Interact _returnvalue_2))

(event Game|Damage|EventAnyDamage
  (params (Damage :type Float%20%28single-precision%29) (DamageType :type Damage%20Type%20Object%20Reference) (InstigatedBy :type Controller%20Object%20Reference) (DamageCauser :type Actor%20Object%20Reference))
  (bind _output_get (Variables|Default|SetM_CurrentHealth (Math|Float|Clamp(Float) (- (Variables|Default|GetM_CurrentHealth) Damage) 0.0 (Variables|Default|GetM_MaxHealth))))
  (Development|PrintString (Utilities|String|ToString(Float) _output_get))
  (if (== _output_get 0.0)
    (CallFunction|Die)))

(fn ConstructionScript)

(fn IsDead
  (return false))

(fn TakeDamage
  (params (DamageInfo :type S%20Damage%20Info%20Structure))
  (bind _wasdamaged_ (Class|BPDamagable|TakeDamage(Message) (Variables|Default|GetBPC_Damage) DamageInfo))
  (return _wasdamaged_))

(fn Heal
  (params (Amount :type Float%20%28double-precision%29))
  (return 0.0))

(fn GetMaxHealth
  (bind _maxhealth (Class|BPDamagable|GetMaxHealth(Message) (Variables|Default|GetBPC_Damage)))
  (return _maxhealth))

(fn GetCurrentHealth
  (bind _health (Class|BPDamagable|GetCurrentHealth(Message) (Variables|Default|GetBPC_Damage)))
  (return _health))

(fn Civil
  (return self))