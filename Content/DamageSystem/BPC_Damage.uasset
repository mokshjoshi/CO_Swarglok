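; BPC_Damage is a damage component that manages health, healing, blocking and death for its owner.
; Heal restores health up to a maximum while alive.
; TakeDamage uses the CanBeDamaged macro to route a damage info struct to block, damage or ignore, based on death, invincibility and blocking.
; It then fires blocked, death or damage-response callbacks, the last only when interruptible or forced, and prints debug output.
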(event EventBeginPlay)

(event EventTick
  (params (DeltaSeconds :type Float%20%28single-precision%29)))

(fn Heal
  (params (Amount :type Float%20%28double-precision%29))
  (if (not (Variables|Default|GetIs%20Dead?))
    (bind _output_get (Variables|Default|SetHealth (Math|Float|Clamp(Float) (+ (Variables|Default|GetHealth) Amount) 0.0 (Variables|Default|GetMaxHealth))))
    (return _output_get)))

(fn TakeDamage
  (params (DamageInfo :type S%20Damage%20Info%20Structure))
  (Development|PrintString "DAMAGEEEEEEE")
  (Utilities|CanbeDamaged (.shoulddamageinvencible DamageInfo) (.canbeblocked DamageInfo)
    (:Block%20Damage
      (Default|CallOnBlocked (.canbeparried DamageInfo))
      (return false))
    (:Do%20Damage
      (bind _output_get (Variables|Default|SetHealth (- (Variables|Default|GetHealth) (.amount DamageInfo))))
      (Development|PrintString (Utilities|String|ToString(Float) _output_get))
      (if (<= _output_get 0.0)
        (Variables|Default|SetIs%20Dead? true)
        (Default|CallOnDeath)
        (return true)
        (elif (or (Variables|Default|GetIs%20Intrruptable?) (.shouldforceinterupt DamageInfo))
          (Default|CallOnDamageResonse (.damageresponse DamageInfo))
          (return true))))
    (:No%20Damage
      (return false))))